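; BP_CameraPawn is a pawn that generates a square tile grid of ground actors when play begins.
; NewFunction loops over GridSize squared indices, stepping row and column offsets at 100-unit spacing and recording each position in GroundPoints.
; The GroundTypes entry at each index selects between two spawn branches that place an actor at that point.
; Despite the name, the graphs show no active camera logic.
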(event `self.ReceiveBeginPlay`
  (`self.NewFunction`))

(fn `NewFunction`
  (bind _gridsize (`self.GridSize`))
  (bind _returnvalue (`KismetMathLibrary.Conv_IntToDouble` (* (`self.YOffset`) 100)))
  (bind _returnvalue_2 (`KismetMathLibrary.Conv_IntToDouble` (* (`self.XOffset`) 100)))
  (bind _returnvalue_3 (`KismetMathLibrary.MakeTransform` (`KismetMathLibrary.MakeVector` _returnvalue _returnvalue_2)))
  (for _index (range (* _gridsize _gridsize))
    (if (== (mod _index (`self.GridSize`)) 0)
      (bind _output_get (set `self.YOffset` (`self.YOffset`)))
      (`/Engine/EditorBlueprintResources/StandardMacros.DecrementInt` _output_get
        (:`  `
          (set `self.XOffset` 0)))
      (else
        (bind _output_get_2 (set `self.XOffset` (`self.XOffset`)))
        (`/Engine/EditorBlueprintResources/StandardMacros.IncrementInt` _output_get_2
          (:`  `
            _))))
    (`KismetArrayLibrary.Array_Add` (`self.GroundPoints`) (`KismetMathLibrary.MakeVector` _returnvalue _returnvalue_2))
    (switch `int` (`|GetArrayItem` (`self.GroundTypes`) _index)
      (:`0`
        (`|SpawnActorFromClass` "/Game/StartContent/AlmejaStudio/Code/BluePrints/BP_Practice/BP_Grass.BP_Grass_C" _returnvalue_3 "Undefined" "MultiplyWithRoot" null null))
      (:`1`
        (`|SpawnActorFromClass` "/Game/StartContent/AlmejaStudio/Code/BluePrints/BP_Practice/BPGround.BPGround_C" _returnvalue_3 "Undefined" "MultiplyWithRoot" null null)))))

(fn `UserConstructionScript`)